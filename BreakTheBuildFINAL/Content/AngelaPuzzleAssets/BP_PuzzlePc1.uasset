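; BP_PuzzlePc1 is a puzzle piece actor that highlights when the first-person character is nearby and can be picked or attached through interaction.
; Box overlap swaps the PuzzlePc material to Coin_m on entry, unless already selected, and restores Mat_PuzzleColours on exit.
; PuzzleInteract attaches the Box to a supplied target point with world transforms kept, sets BeenSelected to suppress further highlighting, and restores the normal material.
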(event `self.Box.OnComponentBeginOverlap`
  (params (OverlappedComponent :type "PrimitiveComponent Object Reference") (OtherActor :type "Actor Object Reference") (OtherComp :type "PrimitiveComponent Object Reference") (OtherBodyIndex :type Integer) (bFromSweep :type Boolean) (SweepResult :type "HitResult Structure (by ref)"))
  (if (not (`self.bBeenSelected`))
    (cast `/Game/FirstPersonBP/Blueprints/FirstPersonCharacter` OtherActor)
    (`PrimitiveComponent.SetMaterial` (`self.PuzzlePc`) 0 "/Game/ThirdPersonBP/THIRDPERSONFOLDERBP/Items/Gold/Coin_m.Coin_m")))

(event `self.Box.OnComponentEndOverlap`
  (params (OverlappedComponent :type "PrimitiveComponent Object Reference") (OtherActor :type "Actor Object Reference") (OtherComp :type "PrimitiveComponent Object Reference") (OtherBodyIndex :type Integer))
  (cast `/Game/FirstPersonBP/Blueprints/FirstPersonCharacter` OtherActor)
  (`PrimitiveComponent.SetMaterial` (`self.PuzzlePc`) 0 "/Game/AngelaPuzzleAssets/Mat_PuzzleColours.Mat_PuzzleColours"))

(fn `PuzzleInteract`
  (params (TargetPoint :type "SceneComponent Object Reference"))
  (returns (Val :type Boolean))
  (`SceneComponent.K2_AttachToComponent` (`self.Box`) TargetPoint "None" "KeepWorld" "KeepWorld" "KeepWorld" true)
  (set `self.bBeenSelected` true)
  (`PrimitiveComponent.SetMaterial` (`self.PuzzlePc`) 0 "/Game/AngelaPuzzleAssets/Mat_PuzzleColours.Mat_PuzzleColours")
  (return false))

(fn `UserConstructionScript`
  (`parent.UserConstructionScript`))