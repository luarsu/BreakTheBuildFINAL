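; BP_PuzzleSlots is a puzzle actor whose PuzzlePc component snaps to a target position through mouse interaction.
; Left-click and cursor-over events set flags, though CursorDown is never cleared here.
; When CheckAttached fires with both flags set, it disables physics, moves PuzzlePc to ClosestTarget and marks it active.
; The construction script tints PuzzlePc with a per-instance Colour through a dynamic material.
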(event `Key|LeftMouseButton`
  (params (Key :type "Key Structure"))
  (:`Pressed`
    (set `self.CursorDown` true)))

(event `self.ReceiveActorBeginCursorOver`
  (set `self.CursorHover` true))

(event `self.ReceiveActorEndCursorOver`
  (set `self.CursorHover` false))

(event `Check Attached`
  (bind _puzzlepc (`self.PuzzlePc`))
  (if (and (`self.CursorDown`) (`self.CursorHover`))
    (`PrimitiveComponent.SetSimulatePhysics` _puzzlepc false)
    (`SceneComponent.K2_SetWorldLocation` _puzzlepc (`SceneComponent.K2_GetComponentLocation` (`self.ClosestTarget`)) false false)
    (set `self.IsActive` true)))

(fn `UserConstructionScript`
  (bind _returnvalue (`PrimitiveComponent.CreateDynamicMaterialInstance` (`self.PuzzlePc`) 0 "/Game/AngelaPuzzleAssets/Textures/Mat_PuzzleColours.Mat_PuzzleColours"))
  (bind _output_get (set `self.DynamicMaterial` _returnvalue))
  (`MaterialInstanceDynamic.SetVectorParameterValue` _output_get "Colour" (`self.Colour`)))