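; Puzzle piece actor that flips when the FirstPersonCharacter overlaps its Box trigger.
; The overlap plays a timeline whose PuzzleTurn value sets Option1's relative pitch, as the Lerp alpha stays at zero; end overlap does nothing.
; The construction script gives Option1 and Option2 dynamic instances of Mat_PuzzleColours, tinted by Colour1 and Colour2.
; PuzzleInteract is a stub that always returns false.
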(event `self.Box.OnComponentBeginOverlap`
  (params (OverlappedComponent :type "PrimitiveComponent Object Reference") (OtherActor :type "Actor Object Reference") (OtherComp :type "PrimitiveComponent Object Reference") (OtherBodyIndex :type Integer) (bFromSweep :type Boolean) (SweepResult :type "HitResult Structure (by ref)"))
  (bind _option1 (`self.Option1`))
  (if (== (`GameplayStatics.GetObjectClass` OtherActor) "/Game/FirstPersonBP/Blueprints/FirstPersonCharacter.FirstPersonCharacter_C")
    (bind (_direction _puzzleturn) (`Timeline|Timeline_0`)
      (:`Update`
        (`SceneComponent.K2_SetRelativeRotation` _option1 (`KismetMathLibrary.MakeRotator` 0.0 (`KismetMathLibrary.Lerp` _puzzleturn (.pitch (`SceneComponent.RelativeRotation` _option1)))) false false)))))

(event `self.Box.OnComponentEndOverlap`
  (params (OverlappedComponent :type "PrimitiveComponent Object Reference") (OtherActor :type "Actor Object Reference") (OtherComp :type "PrimitiveComponent Object Reference") (OtherBodyIndex :type Integer)))

(fn `PuzzleInteract`
  (params (TargetPoint :type "SceneComponent Object Reference"))
  (returns (Val :type Boolean))
  (return false))

(fn `UserConstructionScript`
  (bind _returnvalue (`PrimitiveComponent.CreateDynamicMaterialInstance` (`self.Option1`) 0 "/Game/AngelaPuzzleAssets/Mat_PuzzleColours.Mat_PuzzleColours"))
  (bind _output_get (set `self.DynamicMaterial1` _returnvalue))
  (`MaterialInstanceDynamic.SetVectorParameterValue` _output_get "Colour" (`self.Colour1`))
  (bind _returnvalue_2 (`PrimitiveComponent.CreateDynamicMaterialInstance` (`self.Option2`) 0 "/Game/AngelaPuzzleAssets/Mat_PuzzleColours.Mat_PuzzleColours"))
  (bind _output_get_2 (set `self.DynamicMaterial2` _returnvalue_2))
  (`MaterialInstanceDynamic.SetVectorParameterValue` _output_get_2 "Colour" (`self.Colour2`)))