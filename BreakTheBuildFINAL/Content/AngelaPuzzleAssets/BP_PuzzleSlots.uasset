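; Puzzle slot actor that tracks cursor interaction to detach and shows a configurable colour on its puzzle piece component.
; The construction script creates a dynamic material from Mat_PuzzleColours on PuzzlePc and sets its Colour parameter.
; Cursor overlap events toggle a hover flag, while a left mouse press sets a cursor-down flag that these graphs never clear.
; When CheckAttached is called with both flags true, it sets Attached to false.
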(event `Key|LeftMouseButton`
  (params (Key :type "Key Structure"))
  ;[1 1 1] Attachment Event
  (:`Pressed`
    (set `self.CursorDown` true)))

(event `self.ReceiveActorBeginCursorOver`
  ;[1 1 1] Attachment Event
  (set `self.CursorHover` true))

(event `Check Attached`
  ;[1 1 1] Attachment Event
  (if (and (`self.CursorHover`) (`self.CursorDown`))
    (`self.SetAttached` false)))

(event `self.ReceiveActorEndCursorOver`
  ;[1 1 1] Attachment Event
  (set `self.CursorHover` false))

(fn `UserConstructionScript`
  (bind _returnvalue (`PrimitiveComponent.CreateDynamicMaterialInstance` (`self.PuzzlePc`) 0 "/Game/AngelaPuzzleAssets/Mat_PuzzleColours.Mat_PuzzleColours"))
  (bind _output_get (set `self.DynamicMaterial` _returnvalue))
  (`MaterialInstanceDynamic.SetVectorParameterValue` _output_get "Colour" (`self.Colour`)))