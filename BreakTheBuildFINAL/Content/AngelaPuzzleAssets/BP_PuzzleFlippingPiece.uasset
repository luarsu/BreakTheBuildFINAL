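; BP_PuzzleFlippingPiece is a puzzle piece that flips when the first-person character enters its box with the left mouse button held.
; The mouse input sets a Clicked flag, which is checked only on begin overlap before playing a timeline that drives the roll of Option1.
; The construction script gives Option2 a dynamic Mat_PuzzleColours material tinted by the Colour1 variable.
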(event `Key|LeftMouseButton`
  (params (Key :type "Key Structure"))
  (:`Pressed`
    (set `self.bClicked` true))
  (:`Released`
    (set `self.bClicked` false)))

(event `self.Box.OnComponentBeginOverlap`
  (params (OverlappedComponent :type "PrimitiveComponent Object Reference") (OtherActor :type "Actor Object Reference") (OtherComp :type "PrimitiveComponent Object Reference") (OtherBodyIndex :type Integer) (bFromSweep :type Boolean) (SweepResult :type "HitResult Structure (by ref)"))
  (bind _option1 (`self.Option1`))
  (if (and (== (`GameplayStatics.GetObjectClass` OtherActor) "/Game/FirstPersonBP/Blueprints/FirstPersonCharacter.FirstPersonCharacter_C") (`self.bClicked`))
    (bind (_direction _puzzleturn) (`Timeline|Timeline_0`)
      (:`Update`
        (`SceneComponent.K2_SetRelativeRotation` _option1 (`KismetMathLibrary.MakeRotator` _puzzleturn (.pitch (`SceneComponent.RelativeRotation` _option1)) (.yaw (`SceneComponent.RelativeRotation` _option1))) false false)))))

(event `self.Box.OnComponentEndOverlap`
  (params (OverlappedComponent :type "PrimitiveComponent Object Reference") (OtherActor :type "Actor Object Reference") (OtherComp :type "PrimitiveComponent Object Reference") (OtherBodyIndex :type Integer)))

(fn `UserConstructionScript`
  (bind _returnvalue (`PrimitiveComponent.CreateDynamicMaterialInstance` (`self.Option2`) 0 "/Game/AngelaPuzzleAssets/Mat_PuzzleColours.Mat_PuzzleColours"))
  (bind _output_get (set `self.DynamicMaterial1` _returnvalue))
  (`MaterialInstanceDynamic.SetVectorParameterValue` _output_get "Colour" (`self.Colour1`)))